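; Ball actor that drives life loss and the game-over condition through the shared GameInstance_BP.
; Hits on the Ball component play a sound and set a Timer flag, while overlaps call LifeDecrese on the game instance and clear it.
; Tick polls CurrentLife and, at or below a threshold, shows the game-over widget with cursor and UI-only input, then destroys the ball.
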(event `self.ReceiveTick`
  (params (DeltaSeconds :type "Float (single-precision)"))
  (bind _returnvalue (`GameplayStatics.GetPlayerController` 0))
  (if (<= (`/Game/Blueprint/GameInstance_BP.CurrentLife` (`self.GameInstance`)) 10.0)
    (bind _returnvalue_2 (`|CreateWidget` "/Game/Widget/GameOverWidget.GameOverWidget_C"))
    (`UserWidget.AddToViewport` _returnvalue_2 0)
    (set `PlayerController.bShowMouseCursor` true _returnvalue)
    (`WidgetBlueprintLibrary.SetInputMode_UIOnlyEx` _returnvalue)
    (`self.K2_DestroyActor`)))

(event `self.ReceiveBeginPlay`
  (bind _asgame_instance_bp (cast `/Game/Blueprint/GameInstance_BP` (`GameplayStatics.GetGameInstance`)))
  (set `self.GameInstance` _asgame_instance_bp))

(event `self.Ball.OnComponentHit`
  (params (HitComponent :type "PrimitiveComponent Object Reference") (OtherActor :type "Actor Object Reference") (OtherComp :type "PrimitiveComponent Object Reference") (NormalImpulse :type "Vector Structure") (Hit :type "HitResult Structure (by ref)"))
  (`GameplayStatics.PlaySound2D` "/Game/Assets/4391_4948-lq.4391_4948-lq")
  (set `self.Timer` true))

(event `self.Ball.OnComponentBeginOverlap`
  (params (OverlappedComponent :type "PrimitiveComponent Object Reference") (OtherActor :type "Actor Object Reference") (OtherComp :type "PrimitiveComponent Object Reference") (OtherBodyIndex :type Integer) (bFromSweep :type Boolean) (SweepResult :type "HitResult Structure (by ref)"))
  (`/Game/Blueprint/GameInstance_BP.LifeDecrese` (`self.GameInstance`))
  (set `self.Timer` false))

(fn `UserConstructionScript`)